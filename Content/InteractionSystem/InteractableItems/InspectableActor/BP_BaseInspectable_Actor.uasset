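; Base interactable actor that lets the player inspect an item up close in a UI overlay.
; Construction copies the item's mesh onto an inspection mesh offset far below, isolated by a SceneCapture2D's show-only list.
; Interact opens the inspect widget, switches input context and registers the actor with the player controller.
; Update events rotate, pan and FOV-zoom the mesh within limits; exiting resets it and restores game input.
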(event `self.Interact`
  (params (Interactor :type "Actor Object Reference"))
  (bind _returnvalue (`GameplayStatics.GetPlayerController` 0))
  (`SceneCaptureComponent.SetCaptureSortPriority` (`self.SceneCaptureComponent2D`) 0)
  (`SceneComponent.SetHiddenInGame` (`self.InspectableMesh`) false false)
  (bind _returnvalue_2 (`|CreateWidget` "/Game/InteractionSystem/InteractableItems/InspectableActor/WB_InspectUI.WB_InspectUI_C"))
  (bind _output_get (set `self.InspectUI` _returnvalue_2))
  (`UserWidget.AddToViewport` _output_get 0)
  (set `PlayerController.bShowMouseCursor` true _returnvalue)
  (`WidgetBlueprintLibrary.SetInputMode_GameAndUIEx` _returnvalue null "DoNotLock" false)
  (bind _asbp_first_person_player_controller (cast `/Game/FirstPerson/Blueprints/BP_FirstPersonPlayerController` (`GameplayStatics.GetPlayerController` 0)))
  (`/Game/FirstPerson/Blueprints/BP_FirstPersonPlayerController.Update Input Mapping Context` _asbp_first_person_player_controller "/Game/Input/IMC_Inspect.IMC_Inspect")
  (set `/Game/FirstPerson/Blueprints/BP_FirstPersonPlayerController.InspectableActor` self _asbp_first_person_player_controller)
  (`MeshComponent.SetOverlayMaterial` (`self.InspectableMesh`) null))

(event `Update Mesh Zoom`
  (params (Axis :type "Float (double-precision)"))
  ; Update Mesh Zoom
  (set `SceneCaptureComponent2D.FOVAngle` (`KismetMathLibrary.FClamp` (+ (`SceneCaptureComponent2D.FOVAngle` (`self.SceneCaptureComponent2D`)) (* Axis 3.0)) 40.0 120.0) (`self.SceneCaptureComponent2D`)))

(event `Update Mesh Rotation`
  (params (Rotation :type "Vector2D Structure"))
  (bind (_x _y) (`KismetMathLibrary.BreakVector2D` Rotation))
  (bind _inspectablemesh (`self.InspectableMesh`))
  ; Update Mesh Rotation On Mouse Drag
  (`SceneComponent.K2_SetRelativeRotation` _inspectablemesh (`KismetMathLibrary.ComposeRotators` (`SceneComponent.RelativeRotation` _inspectablemesh) (`KismetMathLibrary.MakeRotator` (* _y -5.0) 0.0 (* _x -5.0))) false false))

(event `Update Mesh Location`
  (params (Location :type "Vector2D Structure"))
  (bind (_x _y) (`KismetMathLibrary.BreakVector2D` Location))
  (bind _relativelocation_x (`KismetMathLibrary.BreakVector` (`SceneComponent.RelativeLocation` (`self.InspectableMesh`))))
  (bind (_relativelocation_x_2 _relativelocation_y _relativelocation_z) (`KismetMathLibrary.BreakVector` (`SceneComponent.RelativeLocation` (`self.InspectableMesh`))))
  (bind _x_2 (.x (.location (`self.InspectableDefaultTransform`))))
  (bind _z (.z (.location (`self.InspectableDefaultTransform`))))
  ; Update Mesh Location
  (`SceneComponent.K2_SetRelativeLocation` (`self.InspectableMesh`) (`KismetMathLibrary.MakeVector` (`KismetMathLibrary.FClamp` (+ _relativelocation_x (* _x 2.0)) (- _x_2 60.0) (+ _x_2 60.0)) 0.0 (`KismetMathLibrary.FClamp` (+ (* _y 2.0) _relativelocation_z) (- _z 60.0) (+ _z 60.0))) false false))

(event `Reset Inspectable Mesh`
  (`SceneComponent.K2_SetRelativeTransform` (`self.InspectableMesh`) (`self.InspectableDefaultTransform`) false false)
  (set `SceneCaptureComponent2D.FOVAngle` 90.0 (`self.SceneCaptureComponent2D`))
  (`SceneCaptureComponent.SetCaptureSortPriority` (`self.SceneCaptureComponent2D`) 1))

(event `Exit Inspection Mode`
  (bind _returnvalue (`GameplayStatics.GetPlayerController` 0))
  (`self.Reset Inspectable Mesh`)
  (`SceneComponent.SetHiddenInGame` (`self.InspectableMesh`) true false)
  (`Widget.RemoveFromParent` (`self.InspectUI`))
  (set `PlayerController.bShowMouseCursor` false _returnvalue)
  (`WidgetBlueprintLibrary.SetInputMode_GameOnly` _returnvalue)
  (bind _asbp_first_person_player_controller (cast `/Game/FirstPerson/Blueprints/BP_FirstPersonPlayerController` (`GameplayStatics.GetPlayerController` 0)))
  (`/Game/FirstPerson/Blueprints/BP_FirstPersonPlayerController.Update Input Mapping Context` _asbp_first_person_player_controller "/Game/Input/IMC_Default.IMC_Default")
  (set `/Game/FirstPerson/Blueprints/BP_FirstPersonPlayerController.InspectableActor` null _asbp_first_person_player_controller))

(fn `UserConstructionScript`
  (bind _inspectablemesh (`self.InspectableMesh`))
  (bind _scenecapturecomponent2d (`self.SceneCaptureComponent2D`))
  (bind (_relativelocation_x _relativelocation_y) (`KismetMathLibrary.BreakVector` (`SceneComponent.RelativeLocation` _scenecapturecomponent2d)))
  (bind (_relativelocation_x_2 _relativelocation_y_2) (`KismetMathLibrary.BreakVector` (`SceneComponent.RelativeLocation` _inspectablemesh)))
  (`parent.UserConstructionScript`)
  (`SceneCaptureComponent.ShowOnlyComponent` (`self.SceneCaptureComponent2D`) (`self.InspectableMesh`))
  (`StaticMeshComponent.SetStaticMesh` _inspectablemesh (`StaticMeshComponent.StaticMesh` (`self.ItemMesh`)))
  (`SceneComponent.K2_SetRelativeLocation` _inspectablemesh (`KismetMathLibrary.MakeVector` _relativelocation_x_2 _relativelocation_y_2 -1000.0) false false)
  (`SceneComponent.K2_SetRelativeLocation` _scenecapturecomponent2d (`KismetMathLibrary.MakeVector` _relativelocation_x _relativelocation_y -1000.0) false false)
  (set `self.InspectableDefaultTransform` (`SceneComponent.GetRelativeTransform` (`self.InspectableMesh`))))